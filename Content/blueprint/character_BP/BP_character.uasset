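; BP_character is a Flappy Bird-style Character that flies forward while constantly sinking.
; BeginPlay sets flying movement, and Tick applies steady movement input along positive X and downward Z.
; Touch presses and the move_up axis share one branch that adds upward input scaled by the axis value while Canmove is true.
; Any hit clears Canmove, ending upward control while the drift continues, and prints a debug string.
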(event `self.ReceiveBeginPlay`
  (`CharacterMovementComponent.SetMovementMode` (`self.CharacterMovement`) "MOVE_Flying" 0))

(event `self.ReceiveTick`
  (params (DeltaSeconds :type "Float (single-precision)"))
  (`self.AddMovementInput` (3.0 0.0 -7.0) 0.3))

(event `InputTouch`
  (params (Location :type "Vector Structure") (FingerIndex :type "ETouchIndex Enum"))
  (:`Pressed`
    (if (`self.canmove?`) :!label _label
      (`self.AddMovementInput` (0.0 0.0 7.0) (stale `InputAxis|move_up` AxisValue)))))

(event `InputAxis|move_up`
  (params (AxisValue :type "Float (single-precision)"))
  (goto _label))

(event `self.ReceiveHit`
  (params (MyComp :type "PrimitiveComponent Object Reference") (Other :type "Actor Object Reference") (OtherComp :type "PrimitiveComponent Object Reference") (bSelfMoved :type Boolean) (HitLocation :type "Vector Structure") (HitNormal :type "Vector Structure") (NormalImpulse :type "Vector Structure") (Hit :type "HitResult Structure (by ref)"))
  (set `self.canmove?` false)
  (`KismetSystemLibrary.PrintString` "lalva"))

(fn `UserConstructionScript`)