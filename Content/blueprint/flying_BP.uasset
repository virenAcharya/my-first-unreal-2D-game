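; Player character Blueprint for a Flappy Bird-style flyer, with a flipbook sprite and Flying movement mode.
; BeginPlay shows a level-specific widget until Start is set; Tick then applies constant forward and downward input as fake gravity.
; Held touch repeatedly launches it upward, alongside a move_up axis and jump sound.
; Any Hit stops movement, swaps to the death flipbook, shows the game-over widget and plays game-over sounds.
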(event `self.ReceiveBeginPlay`
  (bind _returnvalue (`GameplayStatics.GetPlayerController` 0))
  (bind _returnvalue_2 (`GameplayStatics.GetPlayerController` 0))
  (`CharacterMovementComponent.SetMovementMode` (`self.CharacterMovement`) "MOVE_Flying" 0)
  ; show level widget
  (bind _returnvalue_3 (`GameplayStatics.GetCurrentLevelName` true))
  (if (`KismetStringLibrary.EqualEqual_StrStr` _returnvalue_3 "level_1")
    (if (not (`self.start?`))
      (bind _returnvalue_4 (`|CreateWidget` "/Game/blueprint/level_1_WB.level_1_WB_C"))
      (`UserWidget.AddToViewport` _returnvalue_4 0)
      (set `PlayerController.bShowMouseCursor` true _returnvalue)
      (`WidgetBlueprintLibrary.SetInputMode_GameAndUIEx` _returnvalue null))
    (elif (not (`self.start?`))
      (bind _returnvalue_5 (`|CreateWidget` "/Game/blueprint/level_2_WB.level_2_WB_C"))
      (`UserWidget.AddToViewport` _returnvalue_5 0)
      (set `PlayerController.bShowMouseCursor` true _returnvalue_2)
      (`WidgetBlueprintLibrary.SetInputMode_GameAndUIEx` _returnvalue_2 null))))

(event `self.ReceiveTick`
  (params (DeltaSeconds :type "Float (single-precision)"))
  ;[0.6448 0.6249 0 0.5] grevity
  (if (`self.start?`)
    (if (`self.canMove?`)
      (`self.AddMovementInput` (4.0 0.0 -7.0) 0.3)
      (if (`self.isTouching?`)
        (`self.LaunchCharacter` (0.0 0.0 250.0) false true)))))

(event `InputTouch`
  (params (Location :type "Vector Structure") (FingerIndex :type "ETouchIndex Enum"))
  ;[1 1 1 0.5] sound for jumping
  (:`Pressed`
    (if (`self.canMove?`) :!label _label
      (if (`self.start?`)
        (`GameplayStatics.PlaySound2D` "/Game/sound/jump_cue.jump_cue" 1.0 1.0 0.0 null null)))))

(event `Key|SpaceBar`
  (params (Key :type "Key Structure"))
  ;[1 1 1 0.5] sound for jumping
  (:`Pressed`
    (goto _label)))

(event `Key|LeftMouseButton`
  (params (Key :type "Key Structure"))
  ;[1 1 1 0.5] sound for jumping
  (:`Pressed`
    (goto _label)))

(event `InputTouch`
  (params (Location :type "Vector Structure") (FingerIndex :type "ETouchIndex Enum"))
  ;[0.1876 0.9407 1 0.5] character jump
  (:`Pressed`
    (if (`self.start?`) :!label _label_2
      (if (`self.canMove?`)
        (`self.AddMovementInput` (0.0 0.0 7.0) (stale `InputAxis|move_up` AxisValue))))))

(event `Key|Android_Volume_Up`
  (params (Key :type "Key Structure"))
  ;[0 0.6791 0.8031 0.5] jump for android
  (:`Pressed`
    (if (`self.canMove?`) :!label _label_3
      (if (`self.start?`)
        (set `self.isTouching?` true))))
  (:`Released`
    (if (`self.canMove?`) :!label _label_4
      (if (`self.start?`)
        (set `self.isTouching?` false)))))

(event `InputTouch`
  (params (Location :type "Vector Structure") (FingerIndex :type "ETouchIndex Enum"))
  ;[0 0.6791 0.8031 0.5] jump for android
  (:`Pressed`
    (goto _label_3))
  (:`Released`
    (goto _label_4)))

(event `InputAxis|move_up`
  (params (AxisValue :type "Float (single-precision)"))
  ;[0.1876 0.9407 1 0.5] character jump
  (goto _label_2))

(event `self.ReceiveHit`
  (params (MyComp :type "PrimitiveComponent Object Reference") (Other :type "Actor Object Reference") (OtherComp :type "PrimitiveComponent Object Reference") (bSelfMoved :type Boolean) (HitLocation :type "Vector Structure") (HitNormal :type "Vector Structure") (NormalImpulse :type "Vector Structure") (Hit :type "HitResult Structure (by ref)"))
  ;[0.3115 0 0 0.5] loose logic
  (set `self.canMove?` false)
  (`PaperFlipbookComponent.SetFlipbook` (`self.Sprite`) "/Game/charcter/flying_monster/Death_mon.Death_mon")
  (bind _returnvalue (`|CreateWidget` "/Game/blueprint/gameOver_WB.gameOver_WB_C"))
  (`UserWidget.AddToViewport` _returnvalue 0)
  (set `PlayerController.bShowMouseCursor` true (`GameplayStatics.GetPlayerController` 0))
  (set `self.canMove?` false)
  (`self.gameOver`))

(event `gameOver`
  ;[0.15 0 0 0.5] game over sound
  (if (not (`self.canMove?`))
    (`GameplayStatics.PlaySound2D` "/Game/sound/gameoverCUE.gameoverCUE" 1.0 1.0 0.0 null null)
    (`KismetSystemLibrary.Delay` 1.0)
    (`GameplayStatics.PlaySound2D` "/Game/sound/gameoverVCUE.gameoverVCUE" 1.0 1.0 0.0 null null)))

(fn `UserConstructionScript`)